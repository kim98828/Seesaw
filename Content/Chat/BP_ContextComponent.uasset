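; BP_ContextComponent is a component that shows a context menu for party actions and handles the selected option.
; ShowMenu clears any open menu, then creates a ContextMenuWidget from the given options and remembers the caller as instigator.
; OnOptionSelected gets the local player's inventory component and calls its server party functions for inviting, leaving, promoting or kicking.
; The target comes from the instigator, either a character or a party member widget.
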(event EventBeginPlay)

(event EventTick
  (params (DeltaSeconds :type Float%20%28single-precision%29)))

(fn OnOptionSelected
  (params (Option :type E_Context%20Enum :default "NewEnumerator0"))
  (bind _returnvalue (Game|GetPlayerController 0))
  (Variables|Default|SetMenuRef 0)
  (Class|BPIConttrollerInterface|ControllerGetControlledPawnRef(Message) _returnvalue)
  (bind _inv (Class|BPIConttrollerInterface|ControllerGetInventoryComponent(Message) _returnvalue))
  (bind _output_get (LocalVariables|SetInvComp _inv))
  (switch Utilities|FlowControl|Switch|SwitchonE_Context Option
    (:NewEnumerator0
      (Default|SERVERSendPartyRequest _output_get (.AsBP%20Deajin%20Character (Utilities|Casting|CastToBP_DeajinCharacter (Variables|Default|GetMenuInstigator)))))
    (:NewEnumerator1
      (Default|ServerLeaveParty _output_get))
    (:NewEnumerator2
      (bind _asparty_member_widget (Utilities|Casting|CastToPartyMemberWidget (Variables|Default|GetMenuInstigator)))
      (Default|SERVERSetNewLeader _output_get (Variables|/Game/Chat/PartyMemberWidget.PartyMemberWidget_C|GetActorOwner _asparty_member_widget)))
    (:NewEnumerator3
      (bind _asparty_member_widget_2 (Utilities|Casting|CastToPartyMemberWidget (Variables|Default|GetMenuInstigator)))
      (Default|SERVERPartyKickPlayer _output_get (Variables|/Game/Chat/PartyMemberWidget.PartyMemberWidget_C|GetActorOwner _asparty_member_widget_2)))))

(fn ShowMenu
  (params (Option :type Array%20of%20E_Context%20Enums :default "NewEnumerator0") (Caller :type Object%20Object%20Reference))
  (Utilities|FlowControl|Sequence
    (:then_0
      (CallFunction|RemoveMenu))
    (:then_1
      (if (> (Utilities|Array|Length Option) 0)
        (bind _returnvalue (UserInterface|CreateWidget "/Game/Chat/ContextMenuWidget.ContextMenuWidget_C" 0 Option self))
        (bind _output_get (Variables|Default|SetMenuRef _returnvalue))
        (Default|Init _output_get)
        (UserInterface|Viewport|AddtoViewport _returnvalue 0)
        (Variables|Default|SetMenuInstigator Caller)))
    (:then_2
      (return))))

(fn RemoveMenu
  (Utilities|FlowControl|Sequence
    (:then_1
      (Variables|Default|SetMenuInstigator 0)
      (Utilities|IsValid (Variables|Default|GetMenuRef)
        (:Is%20Valid
          (Widget|RemovefromParent (Variables|Default|GetMenuRef))
          (Variables|Default|SetMenuRef 0)
          (return true))))
    (:then_2
      (return false))))