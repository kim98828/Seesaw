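; Player controller component that creates the in-game HUD for the local player and handles party and classroom-entry requests.
; Party SERVER/CLIENT events drive invites with a confirmation popup, accept, leave with leader handoff, kick and delegation.
; Membership and leader state are read and written on each member's controller through interface messages, without direct class references.
; Classroom entry validates the class name, round-trips through the target's component, and currently only prints the result.
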(event EventBeginPlay
  (bind _asplayer_controller (Utilities|Casting|CastToPlayerController (Components|GetOwner)))
  (bind _output_get (Variables|Default|SetControllerOwner _asplayer_controller))
  (if (Pawn|IsLocalController _output_get)
    (|CreateInventory)))

(event EventTick
  (params (DeltaSeconds :type Float%20%28single-precision%29)))

(fn GetControlledPawn
  (bind _actorref (Class|BPIConttrollerInterface|ControllerGetControlledPawnRef(Message) (Components|GetOwner)))
  (return _actorref))

(fn HandleLeaveParty
  (bind _returnvalue (Components|GetOwner))
  (bind _result (Class|BPIConttrollerInterface|ControllerHasParty(Message) _returnvalue))
  (if _result
    (bind _result_2 (Class|BPIConttrollerInterface|ControllerIsPartyLeader(Message) _returnvalue))
    (bind _member (Class|BPIConttrollerInterface|ControllerGetPartyMembers(Message) _returnvalue))
    (for _array_element _member
      (if (Utilities|IsValid _array_element)
        (Utilities|FlowControl|Sequence
          (:then_0
            (Utilities|FlowControl|DoOnce false
              (:Completed
                (LocalVariables|SetNextPartyLeader _array_element))))
          (:then_1
            (bind _playercontrollerref (Class|BPICharaterInterFace|CharaterGetControllerRef(Message) _array_element))
            (Class|BPIConttrollerInterface|ControllerRemovePartyMember(Message) _playercontrollerref (.AsPawn (Utilities|Casting|CastToPawn (CallFunction|GetControlledPawn))))))))
    (Class|BPIConttrollerInterface|ControllerSetPartyMembers(Message) _returnvalue (Utilities|Array|MakeArray))
    (if _result_2
      (Class|BPICharaterInterFace|CharaterSetIsPartyLeader(Message) _returnvalue false)
      (bind _playercontrollerref_2 (Class|BPICharaterInterFace|CharaterGetControllerRef(Message) (LocalVariables|GetNextPartyLeader)))
      (Class|BPIConttrollerInterface|ControllerSetIsPartyLeader(Message) _playercontrollerref_2 true))))

(fn GetControllerRef
  (return (Variables|Default|GetControllerOwner)))

(event Custom|SERVER_SendPartyRequest
  (params (ToPlayer :type Pawn%20Object%20Reference))
  ;[1 1 1] 파티초대 요청
  (Utilities|IsValid ToPlayer
    (:Is%20Valid
      (bind _playercontrollerref (Class|BPICharaterInterFace|CharaterGetControllerRef(Message) ToPlayer))
      (bind _result (Class|BPIConttrollerInterface|ControllerHasParty(Message) _playercontrollerref))
      (bind _result_2 (Class|BPIConttrollerInterface|ControllerIsPartyLeader(Message) _playercontrollerref))
      (if (or _result_2 (not _result))
        (bind _partynum (Class|BPIConttrollerInterface|ControllerHasParty(Message) (Game|Player|GetPlayerPawn 0)))
        (if (and (not _result) (< _partynum (Variables|Default|GetMaxPartyMembers)))
          (bind _inv (Class|BPICharaterInterFace|CharaterGetInventoryComponent(Message) ToPlayer))
          (CallFunction|CLIENTonPartyInvite _inv (CallFunction|GetControlledPawn))
          (else
            (Development|PrintString (select (< _partynum (Variables|Default|GetMaxPartyMembers)) "이미 파티에 가입되어있습니다." "파티가 가득찼습니다"))))
        (else
          (Development|PrintString "You're not the party leader!"))))))

(event Custom|CLIENT_OnPartyInvite
  (params (PlayerRef :type Actor%20Object%20Reference))
  (bind _returnvalue (Game|GetPlayerController 0))
  ;[1 1 1] 파티초대 응답
  (bind _playername (Class|ITIntarractInterface|GetActorName(Message) PlayerRef))
  (Utilities|FlowControl|Sequence
    (:then_0
      (Utilities|IsValid (Variables|Default|GetPartyRequest)
        (:Is%20Valid
          (Widget|RemovefromParent (Variables|Default|GetPartyRequest)))))
    (:then_1
      (bind _returnvalue_2 (UserInterface|CreateWidget "/Game/Chat/BP_JigCofirmationWidget.BP_JigCofirmationWidget_C" 0 (Utilities|Text|ToText(String) _playername) "이(가)당신을 파티에 초대합니다."))
      (bind _output_get (Variables|Default|SetPartyRequest _returnvalue_2))
      (UserInterface|Viewport|AddtoViewport _output_get 0)
      (Input|SetInputModeUIOnly _returnvalue 0 "DoNotLock")
      (Variables|/Script/Engine.PlayerController|SetbShowMouseCursor _returnvalue true)
      (EventDispatchers|BindEventtoClosed _returnvalue_2 (delegate Custom|Closed_Event_2)))))

(event Custom|Closed_Event_2
  (bind _returnvalue (Game|GetPlayerController 0))
  ;[1 1 1] 파티초대 응답
  (Input|SetInputModeGameOnly _returnvalue)
  (Variables|/Script/Engine.PlayerController|SetbShowMouseCursor _returnvalue false)
  (Utilities|FlowControl|Sequence
    (:then_0
      (if (Variables|/Game/Chat/BP_JigCofirmationWidget.BP_JigCofirmationWidget_C|GetConfirmed (stale Custom|CLIENT_OnPartyInvite _returnvalue_2))
        (CallFunction|SERVERAcceptPartyRequest (stale Custom|CLIENT_OnPartyInvite PlayerRef))))
    (:then_1
      (Variables|Default|SetPartyRequest 0))))

(event Custom|SERVER_AcceptPartyRequest
  (params (InvitionPlayer :type Actor%20Object%20Reference))
  ;[1 1 1] 파티요청 수락
  (Utilities|IsValid InvitionPlayer
    (:Is%20Valid
      (bind _result (Class|BPIConttrollerInterface|ControllerHasParty(Message) (Components|GetOwner)))
      (bind _playercontrollerref (Class|BPICharaterInterFace|CharaterGetControllerRef(Message) InvitionPlayer))
      (bind (_result_2 _partynum) (Class|BPIConttrollerInterface|ControllerHasParty(Message) _playercontrollerref))
      (if (and (not _result) (< _partynum (Variables|Default|GetMaxPartyMembers)))
        (if _result_2
          _
          (else
            (Class|BPIConttrollerInterface|ControllerSetIsPartyLeader(Message) _playercontrollerref true)))
        (bind (_result_3 _member) (Class|BPIConttrollerInterface|ControllerGetPartyMembers(Message) _playercontrollerref))
        (if _result_3
          (for _array_element _member
            (bind _actorref (Class|BPIConttrollerInterface|ControllerGetControlledPawnRef(Message) _array_element))
            (Class|BPIConttrollerInterface|ControllerAddPartyMember(Message) _actorref (.AsPawn (Utilities|Casting|CastToPawn (CallFunction|GetControlledPawn)))))
          (bind _member_2 (Class|BPIConttrollerInterface|ControllerGetPartyMembers(Message) _playercontrollerref))
          (Class|BPIConttrollerInterface|ControllerSetPartyMembers(Message) (Components|GetOwner) _member_2))
        (Class|BPIConttrollerInterface|ControllerAddPartyMember(Message) _playercontrollerref (.AsPawn (Utilities|Casting|CastToPawn (CallFunction|GetControlledPawn))))
        (Class|BPIConttrollerInterface|ControllerAddPartyMember(Message) (Components|GetOwner) (.AsPawn (Utilities|Casting|CastToPawn InvitionPlayer)))))))

(event Custom|Server_LeaveParty
  ;[1 1 1] 파티나가기
  (CallFunction|HandleLeaveParty))

(event Custom|SERVER_PartyKickPlayer
  (params (PlayerRef :type Actor%20Object%20Reference))
  (bind _returnvalue (Components|GetOwner))
  (bind _aspawn (Utilities|Casting|CastToPawn PlayerRef))
  ;[1 1 1] 파티 강퇴
  (if (!= PlayerRef (Game|Player|GetPlayerPawn 0))
    (bind _result (Class|BPIConttrollerInterface|ControllerIsPartyLeader(Message) _returnvalue))
    (if _result
      (bind _member (Class|BPIConttrollerInterface|ControllerGetPartyMembers(Message) _returnvalue))
      (if (Utilities|Array|ContainsItem _member (.AsPawn (Utilities|Casting|CastToPawn PlayerRef)))
        (for _array_element _member
          (if (!= _array_element PlayerRef)
            (bind _playercontrollerref (Class|BPICharaterInterFace|CharaterGetControllerRef(Message) _array_element))
            (Class|BPIConttrollerInterface|ControllerRemovePartyMember(Message) _playercontrollerref _aspawn)))
        (bind _playercontrollerref_2 (Class|BPICharaterInterFace|CharaterGetControllerRef(Message) PlayerRef))
        (Class|BPIConttrollerInterface|ControllerSetPartyMembers(Message) _playercontrollerref_2 (Utilities|Array|MakeArray))
        (Class|BPIConttrollerInterface|ControllerRemovePartyMember(Message) (Components|GetOwner) _aspawn)))))

(event Custom|SERVER_SetNewLeader
  (params (PlayerRef :type Actor%20Object%20Reference))
  (bind _returnvalue (Components|GetOwner))
  ;[1 1 1] 파티장 위임
  (if (!= PlayerRef (Game|Player|GetPlayerPawn 0))
    (bind _member (Class|BPIConttrollerInterface|ControllerGetPartyMembers(Message) _returnvalue))
    (if (Utilities|Array|ContainsItem _member (.AsPawn (Utilities|Casting|CastToPawn PlayerRef)))
      (Class|BPIConttrollerInterface|ControllerSetIsPartyLeader(Message) _returnvalue false)
      (bind _playercontrollerref (Class|BPICharaterInterFace|CharaterGetControllerRef(Message) PlayerRef))
      (Class|BPICharaterInterFace|CharaterSetIsPartyLeader(Message) _playercontrollerref false))))

(event Custom|SERVER_InToClass
  (params (PlayerToIn :type Actor%20Object%20Reference))
  ;[1 1 1] 강의실 진입
  (Utilities|IsValid PlayerToIn
    (:Is%20Valid
      (bind (_name _vaild) (Class|BPIConttrollerInterface|ControllerGetClassName(Message) (Components|GetOwner)))
      (if _vaild
        (bind _inv (Class|BPICharaterInterFace|CharaterGetInventoryComponent(Message) PlayerToIn))
        (CallFunction|CLIENTonClassin _inv (Game|Player|GetPlayerPawn 0) (Utilities|String|ToString(Name) _name))
        (else
          (Development|PrintString "강의실이 아닙니다."))))))

(event Custom|CLIENT_OnClassIn
  (params (ByPlayerRef :type Actor%20Object%20Reference) (ClassName :type String))
  ;[1 1 1] 강의실진입(강의실 채팅 쓸지말지 If사용)
  (CallFunction|SERVERonClassinResponse ByPlayerRef))

(event Custom|SERVEROnClassInResponse
  (params (InvitedBy :type Actor%20Object%20Reference))
  ;[1 1 1] 강의실들어온처리
  (Development|PrintString "강의실에 입장하였습니다."))